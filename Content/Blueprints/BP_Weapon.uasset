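; BP_Weapon is a hitscan weapon that fires from the player's first-person camera.
; Use calls Shoot when CanShoot is set and ammo remains; otherwise it waits FireRate, then re-enables CanShoot.
; Shoot runs a persistently debug-drawn Camera-channel trace along the view, ignoring the player, clears CanShoot, decrements Ammo and broadcasts the change.
; The trace's hit result is unused, so no damage is applied.
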(event `/Game/Blueprints/Interfaces/Usable.Use`
  (if (and (`self.CanShoot`) (> (`self.Ammo`) 0))
    (`self.Shoot`)
    (else
      (`KismetSystemLibrary.Delay` (`self.FireRate`))
      (`self.ResetShoot`))))

(event `ResetShoot`
  (set `self.CanShoot` true))

(event `Shoot`
  (bind (_start _end) (`self.GetLineTrace`))
  (`KismetSystemLibrary.LineTraceSingle` _start _end "TraceTypeQuery2" false (`|MakeArray` (`GameplayStatics.GetPlayerPawn` 0) :!type "Actor Object Reference") "Persistent")
  (set `self.CanShoot` false)
  (bind _result (`/Engine/EditorBlueprintResources/StandardMacros.DecrementInt` (`self.Ammo`))
    (:`  `
      (`self.OnAmmoChanged` _result))))

(fn `GetLineTrace`
  (returns (Start :type "Vector Structure") (End :type "Vector Structure"))
  (bind _asbp_my_character (cast `/Game/Blueprints/BP_MyCharacter` (`GameplayStatics.GetPlayerPawn` 0)))
  (bind _firstpersoncamera (`/Game/Blueprints/BP_MyCharacter.FirstPersonCamera` _asbp_my_character))
  (bind _returnvalue (`SceneComponent.K2_GetComponentLocation` _firstpersoncamera))
  (return _returnvalue (+ _returnvalue (* (`KismetMathLibrary.GetForwardVector` (`SceneComponent.K2_GetComponentRotation` _firstpersoncamera)) 30000.0))))

(fn `UserConstructionScript`)